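; BP_DeathFlag is a kill trigger that ends the game when the player overlaps its collision component.
; Overlap branches on the other actor's first tag, destroying interactables and dealing massive damage to enemies.
; For the player, it disables input, hides the HUD, applies that damage and blends the view to a repositioned child-actor camera.
; After a short delay, it shows the game-over widget with a cursor and pauses the game.
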(event `self.CollisionComponent.OnComponentBeginOverlap`
  (params (OverlappedComponent :type "PrimitiveComponent Object Reference") (OtherActor :type "Actor Object Reference") (OtherComp :type "PrimitiveComponent Object Reference") (OtherBodyIndex :type Integer) (bFromSweep :type Boolean) (SweepResult :type "HitResult Structure (by ref)"))
  (bind _returnvalue (`GameplayStatics.GetPlayerController` 0))
  (bind _camera (`self.Camera`))
  (switch `name` (`|GetArrayItem` (`Actor.Tags` OtherActor))
    (:`PlayerTag`
      (bind _asbp_third_person_character (cast `/Game/ThirdPerson/Blueprints/BP_ThirdPersonCharacter` OtherActor))
      (bind _output_get (set `self.As BP Third Person Character` _asbp_third_person_character))
      (`self.DisableInput` _output_get (`GameplayStatics.GetPlayerController` 0))
      (`Widget.SetVisibility` (`/Game/ThirdPerson/Blueprints/BP_ThirdPersonCharacter.WP_Hud` _output_get) "Hidden")
      (`GameplayStatics.ApplyDamage` _output_get 3000.0)
      (bind _returnvalue_2 (`self.K2_GetActorLocation` _output_get))
      (`SceneComponent.K2_SetWorldLocation` _camera _returnvalue_2 false false)
      (bind (_returnvalue_roll _returnvalue_pitch _returnvalue_yaw) (`KismetMathLibrary.BreakRotator` (`self.K2_GetActorRotation` _output_get)))
      (bind (_returnvalue_roll_2 _returnvalue_pitch_2) (`KismetMathLibrary.BreakRotator` (`KismetMathLibrary.FindLookAtRotation` (`SceneComponent.RelativeLocation` _camera) _returnvalue_2)))
      (`SceneComponent.K2_SetWorldRotation` _camera (`KismetMathLibrary.MakeRotator` _returnvalue_roll _returnvalue_pitch_2 _returnvalue_yaw) false false)
      (`PlayerController.SetViewTargetWithBlend` (`GameplayStatics.GetPlayerController` 0) (`ChildActorComponent.ChildActor` (`self.Camera`)) 0.75 "VTBlend_Cubic" 0.0 false)
      (`KismetSystemLibrary.Delay` 1.0)
      (bind _returnvalue_3 (`|CreateWidget` "/Game/ThirdPerson/Maps/Amalia/WBP_GameOver.WBP_GameOver_C" _returnvalue))
      (`UserWidget.AddToViewport` _returnvalue_3 0)
      (set `PlayerController.bShowMouseCursor` true _returnvalue)
      (`WidgetBlueprintLibrary.SetInputMode_GameAndUIEx` _returnvalue _returnvalue_3)
      (`GameplayStatics.SetGamePaused` true))
    (:`InteractableTag`
      (`self.K2_DestroyActor` OtherActor))
    (:`EnemyTag`
      (`GameplayStatics.ApplyDamage` OtherActor 3000.0))))

(fn `UserConstructionScript`)