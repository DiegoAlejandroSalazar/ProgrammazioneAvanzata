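; BP_Door is a level-exit door that plays a transition into the next level when the player reaches it.
; FirstTrigger fires OpenDoor once, which sets global time dilation to zero while a timeline swings the door open.
; It then restores time, blends the view to the door, fades out, disables input and auto-walks the player along +X.
; A loading widget follows, and after a delay ChangeLevel opens the next LevelsName entry.
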(event `OpenDoor`
  (`GameplayStatics.SetGlobalTimeDilation` 0.0)
  (bind (_direction _doorkeyframe) (`Timeline|OpenDoorTimeline` :!via `PlayFromStart`)
    (:`Update`
      (`SceneComponent.K2_SetRelativeRotation` (`self.Door`) (`KismetMathLibrary.MakeRotator` 0.0 0.0 (`KismetMathLibrary.Lerp` 0.0 -90.0 _doorkeyframe)) false false))
    (:`Finished`
      (`GameplayStatics.SetGlobalTimeDilation` 1.0)
      (`PlayerController.SetViewTargetWithBlend` (`GameplayStatics.GetPlayerController` 0) self (`self.FadeTime`) "VTBlend_Linear" 0.0 false)
      (`PlayerCameraManager.StartCameraFade` :`self` (`GameplayStatics.GetPlayerCameraManager` 0) :`ToAlpha` 1.0 :`Duration` (`self.FadeTime`) :`bShouldFadeAudio` true :`bHoldWhenFinished` true)
      (`self.DisableInput` (`GameplayStatics.GetPlayerCharacter` 0) (`GameplayStatics.GetPlayerController` 0))
      (`Timeline|MovePlayerForward` :!via `PlayFromStart`
        (:`Update`
          (`Pawn.AddMovementInput` (`GameplayStatics.GetPlayerCharacter` 0) (1.0 0.0 0.0) 0.3 false))
        (:`Finished`
          (bind _returnvalue (`|CreateWidget` "/Game/UiFolder/WP_LoadingScreen.WP_LoadingScreen_C"))
          (`UserWidget.AddToViewport` _returnvalue 0)
          (`KismetSystemLibrary.Delay` 4.0)
          (`self.ChangeLevel`))))))

(event `self.FirstTrigger.OnComponentBeginOverlap`
  (params (OverlappedComponent :type "PrimitiveComponent Object Reference") (OtherActor :type "Actor Object Reference") (OtherComp :type "PrimitiveComponent Object Reference") (OtherBodyIndex :type Integer) (bFromSweep :type Boolean) (SweepResult :type "HitResult Structure (by ref)"))
  (if (== OtherActor (`GameplayStatics.GetPlayerCharacter` 0))
    (`/Engine/EditorBlueprintResources/StandardMacros.DoOnce` false
      (:`Completed`
        (`self.OpenDoor`)))))

(fn `ChangeLevel`
  (bind _levelsname (`self.LevelsName`))
  (bind _returnvalue (`GameplayStatics.GetCurrentLevelName` true))
  (bind _result (`/Engine/EditorBlueprintResources/StandardMacros.IncrementInt` (`KismetArrayLibrary.Array_Find` _levelsname _returnvalue))
    (:`  `
      (`GameplayStatics.OpenLevel` (`KismetStringLibrary.Conv_StringToName` (`|GetArrayItem` _levelsname _result))))))

(fn `UserConstructionScript`)