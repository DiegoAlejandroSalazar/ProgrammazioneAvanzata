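; BP_HealingSpot is a single-use health pickup for the third-person player character.
; Tick bobs its Sphere vertically around the starting height with a sine of time since creation, scaled by Speed and Distance.
; When an actor whose first tag is PlayerTag overlaps Collision, it adds HealingPower to the character's CurrentHealth, capped at MaxHealth, calls UpdateHealth and destroys itself.
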(event `self.ReceiveBeginPlay`
  (bind (_relativelocation_x _relativelocation_y _relativelocation_z) (`KismetMathLibrary.BreakVector` (`SceneComponent.RelativeLocation` (`self.Sphere`))))
  (set `self.Relative Location Z` _relativelocation_z))

(event `self.ReceiveTick`
  (params (DeltaSeconds :type "Float (single-precision)"))
  (`SceneComponent.K2_SetRelativeLocation` (`self.Sphere`) (`KismetMathLibrary.MakeVector` 0.0 0.0 (+ (`self.Relative Location Z`) (* (`KismetMathLibrary.DegSin` (* (`self.GetGameTimeSinceCreation`) (`self.Speed`))) (`self.Distance`)))) false false))

(event `self.Collision.OnComponentBeginOverlap`
  (params (OverlappedComponent :type "PrimitiveComponent Object Reference") (OtherActor :type "Actor Object Reference") (OtherComp :type "PrimitiveComponent Object Reference") (OtherBodyIndex :type Integer) (bFromSweep :type Boolean) (SweepResult :type "HitResult Structure (by ref)"))
  (if (== (`|GetArrayItem` (`Actor.Tags` OtherActor)) "PlayerTag")
    (bind _asbp_third_person_character (cast `/Game/ThirdPerson/Blueprints/BP_ThirdPersonCharacter` OtherActor))
    (bind _maxhealth (`/Game/ThirdPerson/Blueprints/BP_ThirdPersonCharacter.MaxHealth` _asbp_third_person_character))
    (bind _returnvalue (+ (`/Game/ThirdPerson/Blueprints/BP_ThirdPersonCharacter.CurrentHealth` _asbp_third_person_character) (`self.healingPower`)))
    (if (<= _maxhealth _returnvalue)
      (set `/Game/ThirdPerson/Blueprints/BP_ThirdPersonCharacter.CurrentHealth` _maxhealth _asbp_third_person_character)
      (else
        (set `/Game/ThirdPerson/Blueprints/BP_ThirdPersonCharacter.CurrentHealth` _returnvalue _asbp_third_person_character)))
    (`/Game/ThirdPerson/Blueprints/BP_ThirdPersonCharacter.UpdateHealth` _asbp_third_person_character)
    (`self.K2_DestroyActor`)))

(fn `UserConstructionScript`)