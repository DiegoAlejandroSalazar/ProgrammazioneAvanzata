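; Projectile actor that damages and knocks back what it hits.
; On BeginPlay it passes its Velocity variable to ProjectileMovement.
; When Sphere1 overlaps a component tagged PlayerCollision or EnemyTag, it applies damage to the owning actor.
; If that actor is a Character, it launches it along the projectile's forward direction and destroys itself; otherwise the projectile stays alive.
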(event `self.ReceiveBeginPlay`
  (set `MovementComponent.Velocity` (`self.Velocity`) (`self.ProjectileMovement`)))

(event `self.Sphere1.OnComponentBeginOverlap`
  (params (OverlappedComponent :type "PrimitiveComponent Object Reference") (OtherActor :type "Actor Object Reference") (OtherComp :type "PrimitiveComponent Object Reference") (OtherBodyIndex :type Integer) (bFromSweep :type Boolean) (SweepResult :type "HitResult Structure (by ref)"))
  (if (or (`ActorComponent.ComponentHasTag` OtherComp "PlayerCollision") (`ActorComponent.ComponentHasTag` OtherComp "EnemyTag"))
    (`GameplayStatics.ApplyDamage` OtherActor (`self.Damage`))
    (bind _ascharacter (cast `Character` OtherActor))
    (`Character.LaunchCharacter` _ascharacter (+ (* (`self.GetActorForwardVector`) -1.0) (* (`KismetMathLibrary.GetForwardVector` (`self.K2_GetActorRotation`)) 500.0)) false false)
    (`self.K2_DestroyActor`)))

(fn `UserConstructionScript`)