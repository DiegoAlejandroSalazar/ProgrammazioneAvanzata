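; Boss enemy with difficulty-scaled health and damage, and montage events for sweep, pound and spawn-pound attacks.
; Overlapping "Hazard" actors damage it by velocity, boosted when the player's hand is detached, with sparks and hit stop via time dilation.
; Player collision overlaps deal contact damage; both damage paths use timer-reset DoOnce cooldowns.
; Death clears tags, cancels the player's hand if its hit actor is an enemy, and clears the blackboard alive flag.
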(event `self.ReceiveTick`
  (params (DeltaSeconds :type "Float (single-precision)")))

(event `SetupUI`
  ; Setup ui della vita
)

(event `Ded`
  ; Gestione morte nemici
  (`BlackboardComponent.SetValueAsBool` (`self.GetBlackBoard`) "IsAlive?" false))

(event `UpdateHealth`
  ; Setup ui della vita
  (`self.EnemyHealthUpdated` (`self.GetCurrentEnemyHealthPercent`)))

(event `self.ReceiveBeginPlay`
  ; Beginplay e gestione danni
  (`self.SetEnemyDamageAndHealth`)
  (`self.SetupUI`)
  (bind _asbp_third_person_character (cast `/Game/ThirdPerson/Blueprints/BP_ThirdPersonCharacter` (`Controller.K2_GetPawn` (`GameplayStatics.GetPlayerController` 0))))
  (set `self.As BP Third Person Character` _asbp_third_person_character))

(event `self.ReceiveAnyDamage`
  (params (Damage :type "Float (single-precision)") (DamageType :type "DamageType Object Reference") (InstigatedBy :type "Controller Object Reference") (DamageCauser :type "Actor Object Reference"))
  (bind _handcomponent (`/Game/ThirdPerson/HandMechanics/BP_HandHolder.handComponent` (`/Game/ThirdPerson/Blueprints/BP_ThirdPersonCharacter.BP Hand Holder` (`self.As BP Third Person Character`))))
  ; Beginplay e gestione danni
  (bind _output_get (set `self.CurrentEnemyHealth` (- (`self.CurrentEnemyHealth`) Damage)))
  (`self.UpdateHealth`)
  (if (<= _output_get 0.0)
    (`KismetArrayLibrary.Array_Clear` (`self.Tags`))
    (bind _asbp_base_enemy (cast `/Game/Characters/Enemies/BP_BaseEnemy` (`/Game/ThirdPerson/HandMechanics/handComponent.HitActor` _handcomponent))
      (:`then`
        (if true
          (`/Game/ThirdPerson/HandMechanics/handComponent.Cancel` _handcomponent)
          (`self.Ded`)
          (else
            (`self.Ded` :!label _label))))
      (:`CastFailed`
        (goto _label)))))

(event `self.CapsuleComponent.OnComponentBeginOverlap`
  (params (OverlappedComponent :type "PrimitiveComponent Object Reference") (OtherActor :type "Actor Object Reference") (OtherComp :type "PrimitiveComponent Object Reference") (OtherBodyIndex :type Integer) (bFromSweep :type Boolean) (SweepResult :type "HitResult Structure (by ref)"))
  (bind _overlappedactor (`self.OverlappedActor`))
  ; Danno fatto al nemico
  (set `self.OverlappedActor` OtherActor)
  (bind (_outhit _returnvalue) (`KismetSystemLibrary.LineTraceSingle` :`Start` (`self.K2_GetActorLocation`) :`End` (`self.K2_GetActorLocation` (`self.OverlappedActor`)) :`TraceChannel` "TraceTypeQuery1" :`bIgnoreSelf` false))
  (if _returnvalue
    (if (`self.ActorHasTag` (`self.OverlappedActor`) "Hazard")
      (`/Engine/EditorBlueprintResources/StandardMacros.DoOnce` false :!label _label_2
        (:`Completed`
          (`|ExecutionSequence`
            (:`then_0`
              (bind (_bblockinghit _binitialoverlap _time _distance _location _impactpoint _normal _impactnormal) (`GameplayStatics.BreakHitResult` _outhit))
              (`NiagaraFunctionLibrary.SpawnSystemAtLocation` "/Game/NiagaraEffects/SparkEffect/NS_Spark.NS_Spark" _impactpoint (`KismetMathLibrary.Conv_VectorToRotator` _impactnormal) (2.0 2.0 2.0))
              (bind _damage (`self.GetDamage` (`self.OverlappedActor`)))
              (cast `/Game/Characters/Enemies/BP_BaseEnemy` _overlappedactor
                (:`then`
                  (`GameplayStatics.ApplyDamage` _overlappedactor _damage))
                (:`CastFailed`
                  _))
              (`GameplayStatics.ApplyDamage` self _damage)
              (if (> _damage 0.0)
                (`self.StartHitStop`)))
            (:`then_1`
              (`KismetSystemLibrary.K2_SetTimerDelegate` (delegate `ResetDamage`) 1.0))))))))

(event `ResetDamage`
  ; Danno fatto al nemico
  (goto _label_2 :!via `Reset`))

(event `self.Capsule.OnComponentBeginOverlap`
  (params (OverlappedComponent :type "PrimitiveComponent Object Reference") (OtherActor :type "Actor Object Reference") (OtherComp :type "PrimitiveComponent Object Reference") (OtherBodyIndex :type Integer) (bFromSweep :type Boolean) (SweepResult :type "HitResult Structure (by ref)"))
  (bind _returnvalue (`ActorComponent.ComponentHasTag` OtherComp "PlayerCollision"))
  (bind _returnvalue_2 (`KismetStringLibrary.Conv_BoolToString` _returnvalue))
  ; fa danno al player
  (if _returnvalue
    (`KismetSystemLibrary.PrintString` _returnvalue_2)
    (`/Engine/EditorBlueprintResources/StandardMacros.DoOnce` false :!label _label_3
      (:`Completed`
        (`|ExecutionSequence`
          (:`then_0`
            (`GameplayStatics.ApplyDamage` OtherActor (`self.EnemyDamage`)))
          (:`then_1`
            (`KismetSystemLibrary.K2_SetTimerDelegate` (delegate `ResetDamageDealt`) 0.5)))))
    (else
      (`KismetSystemLibrary.PrintString` _returnvalue_2))))

(event `ResetDamageDealt`
  ; fa danno al player
  (goto _label_3 :!via `Reset`))

(event `/Game/Characters/Enemies/Enemy_AIs/BPI_BossInterface.Sweep`
  (set `self.IsAttacking?` true)
  (`|PlayMontage` null "/Game/Characters/Enemies/Animazioni/Boss/AM_BossSweep.AM_BossSweep"
    (:`OnCompleted`
      (set `self.IsAttacking?` false))))

(event `/Game/Characters/Enemies/Enemy_AIs/BPI_BossInterface.SpawnPound`
  (set `self.IsAttacking?` true)
  (`|PlayMontage` null "/Game/Characters/Enemies/Animazioni/Boss/AM_BossSpawnPound.AM_BossSpawnPound"
    (:`OnCompleted`
      (set `self.IsAttacking?` false))))

(event `/Game/Characters/Enemies/Enemy_AIs/BPI_BossInterface.Pound`
  (set `self.IsAttacking?` true)
  (`|PlayMontage` null "/Game/Characters/Enemies/Animazioni/Boss/AM_BossBigPound.AM_BossBigPound"
    (:`OnCompleted`
      (set `self.IsAttacking?` false))))

(fn `EndHitStop`
  (set `Actor.CustomTimeDilation` 1.0 (`self.As BP Third Person Character`))
  (set `self.CustomTimeDilation` 1.0))

(fn `FollowPlayer`
  (returns (NewParam :type Boolean))
  (return false))

(fn `GetCurrentEnemyHealthPercent`
  (returns (HealthPercent :type "Float (double-precision)"))
  (return (/ (`self.CurrentEnemyHealth`) (`self.MaxEnemyHealth`))))

(fn `GetDamage`
  (params (OverlappedActor :type "Actor Object Reference"))
  (returns (Damage :type "Float (double-precision)"))
  (bind _asbp_third_person_game_mode (cast `/Game/ThirdPerson/Blueprints/BP_ThirdPersonGameMode` (`GameplayStatics.GetGameMode`)))
  (if (`/Game/ThirdPerson/Blueprints/BP_ThirdPersonCharacter.Hand Attached?` (`self.As BP Third Person Character`))
    (bind _returnvalue (`KismetMathLibrary.MapRangeClamped` (`KismetMathLibrary.VSize` (`self.GetVelocity` OverlappedActor)) 0.0 2000.0 0.0 (* (`/Game/ThirdPerson/Blueprints/BP_ThirdPersonGameMode.Difficulty` _asbp_third_person_game_mode) 60.0)))
    (return _returnvalue)
    (else
      (return (* _returnvalue 1.5)))))

(fn `SetEnemyDamageAndHealth`
  (bind _asbp_third_person_game_mode (cast `/Game/ThirdPerson/Blueprints/BP_ThirdPersonGameMode` (`GameplayStatics.GetGameMode`)))
  (`|ExecutionSequence`
    (:`then_0`
      (bind _difficulty (`/Game/ThirdPerson/Blueprints/BP_ThirdPersonGameMode.Difficulty` _asbp_third_person_game_mode))
      (bind _output_get (set `self.MaxEnemyHealth` (* (`self.DefaultMaxEnemyHealth`) _difficulty)))
      (set `self.CurrentEnemyHealth` _output_get))
    (:`then_1`
      (set `self.EnemyDamage` (* _difficulty (`self.DefaultEnemyDamage`))))))

(fn `StartHitStop`
  (set `Actor.CustomTimeDilation` 0.0 (`self.As BP Third Person Character`))
  (set `self.CustomTimeDilation` 0.0)
  (`KismetSystemLibrary.K2_SetTimer` null "EndHitStop" 0.1))

(fn `UserConstructionScript`)