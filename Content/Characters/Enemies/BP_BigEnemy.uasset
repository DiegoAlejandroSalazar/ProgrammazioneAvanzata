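; Big enemy Blueprint that extends a parent enemy, scaling max health and damage by 1.5 on BeginPlay and starting at full health.
; Its own overlap events are empty, leaving the player-collision check and hit sound unreachable.
; That orphaned chain feeds a DoOnce that applies damage and sets a half-second timer to reset itself, so this contact attack never runs here.
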(event `self.ReceiveBeginPlay`
  (`parent.ReceiveBeginPlay`)
  (bind _output_get (set `self.MaxEnemyHealth` (* (`self.MaxEnemyHealth`) 1.5)))
  (set `self.CurrentEnemyHealth` _output_get)
  (set `self.EnemyDamage` (* (`self.EnemyDamage`) 1.5)))

(event `self.ReceiveActorBeginOverlap`
  (params (OtherActor :type "Actor Object Reference")))

(event `self.DetectionHitBox.OnComponentBeginOverlap`
  (params (OverlappedComponent :type "PrimitiveComponent Object Reference") (OtherActor :type "Actor Object Reference") (OtherComp :type "PrimitiveComponent Object Reference") (OtherBodyIndex :type Integer) (bFromSweep :type Boolean) (SweepResult :type "HitResult Structure (by ref)")))

(event `CustomEvent`
  (`/Engine/EditorBlueprintResources/StandardMacros.DoOnce` false :!via `Reset`
    (:`Completed`
      (`|ExecutionSequence`
        (:`then_0`
          (`GameplayStatics.ApplyDamage` (stale `self.DetectionHitBox.OnComponentBeginOverlap` OtherActor) (`self.EnemyDamage`)))
        (:`then_1`
          (`KismetSystemLibrary.K2_SetTimerDelegate` (delegate `CustomEvent`) 0.5))))))

(fn `UserConstructionScript`
  (`parent.UserConstructionScript`))