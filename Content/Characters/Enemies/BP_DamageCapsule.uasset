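; BP_DamageCapsule is a damage hitbox that, as a child actor of BP_BOSS, hurts the player on contact.
; On BeginPlay it caches the parent boss to read its EnemyDamage value.
; Overlaps with components tagged PlayerCollision apply that damage and spawn a cartoon smoke explosion at the hit actor.
; A DoOnce gate, reset by a short timer, throttles repeated hits.
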(event `self.CollisionComponent.OnComponentBeginOverlap`
  (params (OverlappedComponent :type "PrimitiveComponent Object Reference") (OtherActor :type "Actor Object Reference") (OtherComp :type "PrimitiveComponent Object Reference") (OtherBodyIndex :type Integer) (bFromSweep :type Boolean) (SweepResult :type "HitResult Structure (by ref)"))
  (bind (_returnvalue_location _returnvalue_rotation) (`KismetMathLibrary.BreakTransform` (`self.GetTransform` OtherActor)))
  ; fa danno al player
  (if (`ActorComponent.ComponentHasTag` OtherComp "PlayerCollision")
    (`/Engine/EditorBlueprintResources/StandardMacros.DoOnce` false :!label _label
      (:`Completed`
        (`|ExecutionSequence`
          (:`then_0`
            (`GameplayStatics.ApplyDamage` OtherActor (`/Game/Characters/Enemies/BP_BOSS.EnemyDamage` (`self.As BP BOSS`)))
            (`NiagaraFunctionLibrary.SpawnSystemAtLocation` "/Game/NiagaraEffects/CartoonExplosion/NS_CartoonExplosionSmoke.NS_CartoonExplosionSmoke" _returnvalue_location _returnvalue_rotation (10.0 10.0 10.0)))
          (:`then_1`
            (`KismetSystemLibrary.K2_SetTimerDelegate` (delegate `ResetDamageDealt`) 0.5)))))))

(event `ResetDamageDealt`
  ; fa danno al player
  (goto _label :!via `Reset`))

(event `self.ReceiveBeginPlay`
  (bind _asbp_boss (cast `/Game/Characters/Enemies/BP_BOSS` (`self.GetParentActor`)))
  (set `self.As BP BOSS` _asbp_boss))

(fn `UserConstructionScript`)