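; Enemy character with a health bar, a behavior-tree-triggered montage attack and a grab/airborne stun state.
; Tick sets the blackboard's IsStunned while grabbed or moving vertically, and removes its own Hazard tag the first time neither holds.
; Overlap capsules damage it from line-traced Hazard actors with sparks, and damage the player on contact, each throttled by timer-reset DoOnce gates.
; Damage updates the health widget and clears IsEnemyAlive at zero.
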(event `self.ReceiveBeginPlay`
  ; EnemyHealthBarSystem
  (`self.SetupUI`))

(event `SetupUI`
  ; EnemyHealthBarSystem
  (message `/Game/UiFolder/BPI_SetUiOwner.SetUiOwner` (`WidgetComponent.GetUserWidgetObject` (`self.HealthBar`)) self)
  (`self.UpdateHealth`))

(event `self.ReceiveAnyDamage`
  (params (Damage :type "Float (single-precision)") (DamageType :type "DamageType Object Reference") (InstigatedBy :type "Controller Object Reference") (DamageCauser :type "Actor Object Reference"))
  ; EnemyHealthBarSystem
  (bind _output_get (set `self.CurrentEnemyHealth` (- (`self.CurrentEnemyHealth`) Damage)))
  (`self.UpdateHealth`)
  (if (<= _output_get 0.0)
    (set `self.IsEnemyAlive?` false)))

(event `UpdateHealth`
  ; EnemyHealthBarSystem
  (`self.EnemyHealthUpdated` (`self.GetCurrentEnemyHealthPercent`)))

(event `self.ReceiveTick`
  (params (DeltaSeconds :type "Float (single-precision)"))
  (bind (_velocity_x _velocity_y _velocity_z) (`KismetMathLibrary.BreakVector` (`MovementComponent.Velocity` (`self.CharacterMovement`))))
  (if (or (or (< _velocity_z 0.0) (> _velocity_z 0.0)) (`self.IsGrabbed?`))
    (`BlackboardComponent.SetValueAsBool` (`AIBlueprintHelperLibrary.GetBlackboard` (`AIBlueprintHelperLibrary.GetAIController` self)) "IsStunned" true)
    (else
      (`BlackboardComponent.SetValueAsBool` (`AIBlueprintHelperLibrary.GetBlackboard` (`AIBlueprintHelperLibrary.GetAIController` self)) "IsStunned" false)
      (`/Engine/EditorBlueprintResources/StandardMacros.DoOnce` false
        (:`Completed`
          (`KismetArrayLibrary.Array_RemoveItem` (`self.Tags`) "Hazard"))))))

(event `Attack`
  ; Evento di attacco
  (if (not (`self.IsAttacking?`))
    (set `self.IsAttacking?` true)
    (`|PlayMontage` (`self.Mesh`) "/Game/Characters/Enemies/Animazioni/AM_EnemyAttack.AM_EnemyAttack"
      (:`OnCompleted`
        _)
      (:`OnInterrupted`
        _))
    (set `self.IsAttacking?` false)))

(event `AttackCallFromBehaviorTree`
  ; Evento di attacco
  (if (not (`self.IsAttacking?`))
    (`self.Attack`)))

(event `self.CapsuleComponent.OnComponentBeginOverlap`
  (params (OverlappedComponent :type "PrimitiveComponent Object Reference") (OtherActor :type "Actor Object Reference") (OtherComp :type "PrimitiveComponent Object Reference") (OtherBodyIndex :type Integer) (bFromSweep :type Boolean) (SweepResult :type "HitResult Structure (by ref)")))

(event `self.Capsule.OnComponentBeginOverlap`
  (params (OverlappedComponent :type "PrimitiveComponent Object Reference") (OtherActor :type "Actor Object Reference") (OtherComp :type "PrimitiveComponent Object Reference") (OtherBodyIndex :type Integer) (bFromSweep :type Boolean) (SweepResult :type "HitResult Structure (by ref)"))
  ; Danno fatto al nemic ( da vede se fa cusci )
  (bind (_outhit _returnvalue) (`KismetSystemLibrary.LineTraceSingle` (`self.K2_GetActorLocation`) (`self.K2_GetActorLocation` OtherActor) "TraceTypeQuery1"))
  (if _returnvalue
    (`/Engine/EditorBlueprintResources/StandardMacros.DoOnce` false :!label _label
      (:`Completed`
        (`|ExecutionSequence`
          (:`then_0`
            (if (`self.ActorHasTag` OtherActor "Hazard")
              (bind (_bblockinghit _binitialoverlap _time _distance _location _impactpoint _normal _impactnormal) (`GameplayStatics.BreakHitResult` _outhit))
              (`NiagaraFunctionLibrary.SpawnSystemAtLocation` "/Game/NiagaraEffects/SparkEffect/NS_Spark.NS_Spark" _impactpoint (`KismetMathLibrary.Conv_VectorToRotator` _impactnormal))
              (`GameplayStatics.ApplyDamage` self 15.0)))
          (:`then_1`
            (`KismetSystemLibrary.K2_SetTimerDelegate` (delegate `ResetDamage`) 2.0)))))))

(event `ResetDamage`
  ; Danno fatto al nemic ( da vede se fa cusci )
  (goto _label :!via `Reset`))

(event `self.Capsule1.OnComponentBeginOverlap`
  (params (OverlappedComponent :type "PrimitiveComponent Object Reference") (OtherActor :type "Actor Object Reference") (OtherComp :type "PrimitiveComponent Object Reference") (OtherBodyIndex :type Integer) (bFromSweep :type Boolean) (SweepResult :type "HitResult Structure (by ref)"))
  (if (`ActorComponent.ComponentHasTag` OtherComp "PlayerCollision")
    (`/Engine/EditorBlueprintResources/StandardMacros.DoOnce` false :!label _label_2
      (:`Completed`
        (`|ExecutionSequence`
          (:`then_0`
            (`GameplayStatics.ApplyDamage` OtherActor 10.0))
          (:`then_1`
            (`KismetSystemLibrary.K2_SetTimerDelegate` (delegate `ResetDamageDealt`) 0.5)))))))

(event `ResetDamageDealt`
  (goto _label_2 :!via `Reset`))

(fn `GetCurrentEnemyHealthPercent`
  (returns (HealthPercent :type "Float (double-precision)"))
  (return (/ (`self.CurrentEnemyHealth`) (`self.MaxEnemyHealth`))))

(fn `UserConstructionScript`)