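; Ranged enemy child Blueprint that scales inherited stats to less health and more damage, and fires BP_Projectile at the player.
; FireProjectile skips when custom time dilation is zero, then spawns a player-facing projectile carrying the enemy's damage.
; Launch velocity randomly uses either moving-target prediction or a fixed-speed ballistic toss at the player's current position.
; Tick stores a clamped yaw toward the player in Angle and prints it for debugging.
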(event `self.ReceiveBeginPlay`
  (bind _enemydamage (`self.EnemyDamage`))
  (`parent.ReceiveBeginPlay`)
  (bind _output_get (set `self.MaxEnemyHealth` (* (`self.MaxEnemyHealth`) 0.4)))
  (set `self.CurrentEnemyHealth` _output_get)
  (`|VariableSetRef` _enemydamage (* _enemydamage 1.4)))

(event `Fire Projectile`
  (if (!= (`self.CustomTimeDilation`) 0.0)
    (`/Engine/EditorBlueprintResources/StandardMacros.DoOnce` false :!label _label
      (:`Completed`
        (bind _velocity (`self.GetRandomProjectileVelocity`))
        (bind _returnvalue (`|SpawnActorFromClass` "/Game/Actors/BP_Projectile.BP_Projectile_C" (`KismetMathLibrary.MakeTransform` (`SceneComponent.K2_GetComponentLocation` (`self.ProjectileSpawnPos`)) (`KismetMathLibrary.FindLookAtRotation` (`self.K2_GetActorLocation`) (`self.K2_GetActorLocation` (`GameplayStatics.GetPlayerCharacter` 0)))) "AlwaysSpawn" "MultiplyWithRoot" null _velocity null))
        (`/Engine/EditorBlueprintResources/StandardMacros.IsValid` _returnvalue
          (:`Is Valid`
            (set `/Game/Actors/BP_Projectile.Damage` (`self.EnemyDamage`) _returnvalue)
            (goto _label :!via `Reset`))
          (:`Is Not Valid`
            (`KismetSystemLibrary.PrintString` "Hello")))))))

(event `self.ReceiveTick`
  (params (DeltaSeconds :type "Float (single-precision)"))
  (bind _output_get (set `self.Angle` (`KismetMathLibrary.FClamp` (.yaw (`KismetMathLibrary.FindLookAtRotation` (`self.K2_GetActorLocation`) (`self.K2_GetActorLocation` (`self.As BP Third Person Character`)))) -100.0 100.0)))
  (`KismetSystemLibrary.PrintString` (`KismetStringLibrary.Conv_DoubleToString` _output_get)))

(fn `GetRandomProjectileVelocity`
  (returns (Velocity :type "Vector Structure"))
  (if (`KismetMathLibrary.RandomBool`)
    (bind _outlaunchvelocity (`GameplayStatics.SuggestProjectileVelocity_MovingTarget` (`SceneComponent.K2_GetComponentLocation` (`self.ProjectileSpawnPos`)) (`GameplayStatics.GetPlayerCharacter` 0) (0.0 0.0 0.0) -980.0 1.0 "None"))
    (return _outlaunchvelocity)
    (else
      (bind _tossvelocity (`GameplayStatics.BlueprintSuggestProjectileVelocity` (`SceneComponent.K2_GetComponentLocation` (`self.ProjectileSpawnPos`)) (`self.K2_GetActorLocation` (`GameplayStatics.GetPlayerCharacter` 0)) 2000.0 -980.0 "DoNotTrace"))
      (return _tossvelocity))))

(fn `UserConstructionScript`
  (`parent.UserConstructionScript`))