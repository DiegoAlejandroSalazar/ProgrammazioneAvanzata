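; Base enemy AI controller that runs BT_EnemyBehavior on BeginPlay and feeds it sight perception of the player.
; When sight of player pawn 0 updates, it sets TargetActor to the player if sensed and clears it otherwise.
; A successful sighting stores the stimulus location in LastKnownLocation.
; Tick also rewrites LastKnownLocation every frame from the perception event's stimulus output, with no sense or success check.
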(event `self.ReceiveBeginPlay`
  (`self.RunBehaviorTree` "/Game/Characters/Enemies/Enemy_AIs/BT_EnemyBehavior.BT_EnemyBehavior"))

(event `self.AIPerception.OnTargetPerceptionUpdated`
  (params (Actor :type "Actor Object Reference") (Stimulus :type "AIStimulus Structure"))
  (bind (_age _expirationage _strength _stimuluslocation _receiverlocation _tag _bsuccessfullysensed) (break `AIStimulus` Stimulus))
  ; Se percepisce qalcosa controlla che sia il player, se lo è imposta come oggetto il pawn del giocatore altrimenti raggiunge l'ultima posizione in cui l'ha visto
  (bind _returnvalue (`AIPerceptionSystem.GetSenseClassForStimulus` Stimulus))
  (if (and (== _returnvalue "/Script/AIModule.AISense_Sight") (== Actor (`GameplayStatics.GetPlayerPawn` 0)))
    (`BlackboardComponent.SetValueAsObject` (`self.Blackboard`) "TargetActor" (`KismetMathLibrary.SelectObject` (`GameplayStatics.GetPlayerPawn` 0) null _bsuccessfullysensed))
    (if _bsuccessfullysensed
      (`BlackboardComponent.SetValueAsVector` (`self.Blackboard`) "LastKnownLocation" _stimuluslocation))))

(event `self.ReceiveTick`
  (params (DeltaSeconds :type "Float (single-precision)"))
  ; Se percepisce qalcosa controlla che sia il player, se lo è imposta come oggetto il pawn del giocatore altrimenti raggiunge l'ultima posizione in cui l'ha visto
  (`BlackboardComponent.SetValueAsVector` (`self.Blackboard`) "LastKnownLocation" (`.StimulusLocation` (break `AIStimulus` (stale `self.AIPerception.OnTargetPerceptionUpdated` Stimulus)))))

(fn `UserConstructionScript`)