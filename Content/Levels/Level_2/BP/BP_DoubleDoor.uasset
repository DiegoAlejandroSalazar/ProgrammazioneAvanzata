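; Level-exit double door that opens once when the player enters its box with all keys required by the level's MyChangeLevelCheckTriggerBox actors.
; OpenDoor slides the panels with global time dilation at zero, then fades out, walks the player forward, shows a loading screen, resets saved tries and loads the next listed level.
; LookAtDoor plays a cog sequence and briefly cuts input for a camera reveal.
; Both events start counter-rotating gears on Tick.
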(event `self.ReceiveBeginPlay`
  (bind _asbp_third_person_character (cast `/Game/ThirdPerson/Blueprints/BP_ThirdPersonCharacter` (`GameplayStatics.GetPlayerCharacter` 0)))
  (set `self.As BP Third Person Character` _asbp_third_person_character))

(event `LookAtDoor`
  (bind _returnvalue (`GameplayStatics.GetPlayerController` 0))
  (bind _returnvalue_2 (`GameplayStatics.GetPlayerController` 0))
  (bind _outactor (`LevelSequencePlayer.CreateLevelSequencePlayer` "/Game/Levels/Level_2/Sequences/LS_COGS_2.LS_COGS_2"))
  (`MovieSceneSequencePlayer.PlayLooping` (`LevelSequenceActor.SequencePlayer` _outactor) -1)
  (set `self.Finished?` true)
  (`KismetSystemLibrary.PrintString` "Da stoppare i nemici ")
  (`Widget.SetVisibility` (`/Game/ThirdPerson/Blueprints/BP_ThirdPersonCharacter.WP_Hud` (`self.As BP Third Person Character`)) "Hidden")
  (`self.DisableInput` (`self.As BP Third Person Character`) _returnvalue_2)
  (`PlayerController.SetViewTargetWithBlend` _returnvalue_2 self 4.0 "VTBlend_EaseIn" 1.0 false)
  (`KismetSystemLibrary.Delay` 4.0)
  (`PlayerCameraManager.StartCameraFade` :`self` (`GameplayStatics.GetPlayerCameraManager` 0) :`ToAlpha` 1.0 :`Duration` 1.5 :`bHoldWhenFinished` true)
  (`KismetSystemLibrary.Delay` 1.5)
  (`PlayerCameraManager.StartCameraFade` :`self` (`GameplayStatics.GetPlayerCameraManager` 0) :`FromAlpha` 1.0 :`Duration` 1.5)
  (`PlayerController.SetViewTargetWithBlend` _returnvalue (`self.As BP Third Person Character`) 0.0 "VTBlend_EaseIn" 0.0 false)
  (`KismetSystemLibrary.Delay` 1.5)
  (`Widget.SetVisibility` (`/Game/ThirdPerson/Blueprints/BP_ThirdPersonCharacter.WP_Hud` (`self.As BP Third Person Character`)) "Visible")
  (`self.EnableInput` (`self.As BP Third Person Character`) _returnvalue))

(event `self.ReceiveTick`
  (params (DeltaSeconds :type "Float (single-precision)"))
  (bind _returnvalue (`KismetMathLibrary.MakeRotator` (* DeltaSeconds (`self.Speed`))))
  (if (`self.Finished?`)
    (`|ExecutionSequence`
      (:`then_0`
        (`SceneComponent.K2_AddLocalRotation` (`self.Ingranaggio`) (* _returnvalue -1.0) false false)
        (`SceneComponent.K2_AddLocalRotation` (`self.Ingranaggio6`) (* _returnvalue -1.0) false false)
        (`SceneComponent.K2_AddLocalRotation` (`self.Ingranaggio7`) (* _returnvalue -1.0) false false)
        (`SceneComponent.K2_AddLocalRotation` (`self.Ingranaggio3`) (* _returnvalue -1.0) false false))
      (:`then_1`
        (`SceneComponent.K2_AddLocalRotation` (`self.Ingranaggio1`) _returnvalue false false)
        (`SceneComponent.K2_AddLocalRotation` (`self.Ingranaggio5`) _returnvalue false false)
        (`SceneComponent.K2_AddLocalRotation` (`self.Ingranaggio2`) _returnvalue false false)
        (`SceneComponent.K2_AddLocalRotation` (`self.Ingranaggio4`) _returnvalue false false)))))

(event `OpenDoor`
  (bind _returnvalue (`GameplayStatics.GetPlayerCharacter` 0))
  (bind (_relativelocation_x _relativelocation_y _relativelocation_z) (`KismetMathLibrary.BreakVector` (`SceneComponent.RelativeLocation` (`self.Anta_Sinistra`))))
  (bind (_relativelocation_x_2 _relativelocation_y_2 _relativelocation_z_2) (`KismetMathLibrary.BreakVector` (`SceneComponent.RelativeLocation` (`self.Anta_Destra`))))
  (set `self.Finished?` true)
  (`GameplayStatics.SetGlobalTimeDilation` 0.0)
  (bind (_direction _doorkeyframe) (`Timeline|Timeline` :!via `PlayFromStart`)
    (:`Update`
      (`|ExecutionSequence`
        (:`then_0`
          (`SceneComponent.K2_SetRelativeLocation` (`self.Anta_Destra`) (`KismetMathLibrary.MakeVector` _relativelocation_x_2 (`KismetMathLibrary.Lerp` 0.0 90.0 _doorkeyframe) _relativelocation_z_2) false false))
        (:`then_1`
          (`SceneComponent.K2_SetRelativeLocation` (`self.Anta_Sinistra`) (`KismetMathLibrary.MakeVector` _relativelocation_x (`KismetMathLibrary.Lerp` 0.0 -90.0 _doorkeyframe) _relativelocation_z) false false))))
    (:`Finished`
      (`GameplayStatics.SetGlobalTimeDilation` 1.0)
      (`Widget.SetVisibility` (`/Game/ThirdPerson/Blueprints/BP_ThirdPersonCharacter.WP_Hud` (`self.As BP Third Person Character`)) "Hidden")
      (`PlayerController.SetViewTargetWithBlend` (`GameplayStatics.GetPlayerController` 0) self (`self.FadeTime`) "VTBlend_Linear" 0.0 false)
      (`PlayerCameraManager.StartCameraFade` :`self` (`GameplayStatics.GetPlayerCameraManager` 0) :`ToAlpha` 1.0 :`Duration` (`self.FadeTime`) :`bShouldFadeAudio` true :`bHoldWhenFinished` true)
      (set `Actor.bCanBeDamaged` false _returnvalue)
      (`self.DisableInput` _returnvalue (`GameplayStatics.GetPlayerController` 0))
      (`Timeline|Timeline_2` :!via `PlayFromStart`
        (:`Update`
          (`Pawn.AddMovementInput` (`GameplayStatics.GetPlayerCharacter` 0) (1.0 0.0 0.0) 0.3 false))
        (:`Finished`
          (bind _returnvalue_2 (`|CreateWidget` "/Game/UiFolder/WP_LoadingScreen.WP_LoadingScreen_C"))
          (`UserWidget.AddToViewport` _returnvalue_2 0)
          (`KismetSystemLibrary.Delay` 4.0)
          (`self.ChangeLevel`))))))

(event `self.Box.OnComponentBeginOverlap`
  (params (OverlappedComponent :type "PrimitiveComponent Object Reference") (OtherActor :type "Actor Object Reference") (OtherComp :type "PrimitiveComponent Object Reference") (OtherBodyIndex :type Integer) (bFromSweep :type Boolean) (SweepResult :type "HitResult Structure (by ref)"))
  (if (== OtherActor (`GameplayStatics.GetPlayerCharacter` 0))
    (bind _outactors (`GameplayStatics.GetAllActorsOfClass` "/Script/PJ_Prog_Avanzata.MyChangeLevelCheckTriggerBox"))
    (set `self.TotalCurrentKey` 0)
    (set `self.TotalKeyNeeded` 0)
    (for _array_element _outactors
      (set `self.TotalKeyNeeded` (+ (`MyChangeLevelCheckTriggerBox.keysNeeded` _array_element) (`self.TotalKeyNeeded`)))
      (set `self.TotalCurrentKey` (+ (`MyChangeLevelCheckTriggerBox.CurrentKeys` _array_element) (`self.TotalCurrentKey`))))
    (if (== (`self.TotalKeyNeeded`) (`self.TotalCurrentKey`))
      (`/Engine/EditorBlueprintResources/StandardMacros.DoOnce` false
        (:`Completed`
          (`self.OpenDoor`)))
      (else
        (`KismetSystemLibrary.PrintString` "Ti mancano delle chiavi" true true (struct :`R` 1.0 :`B` 0.031819 :`A` 1.0))))))

(fn `ChangeLevel`
  (bind _levelsname (`self.LevelsName`))
  (bind _returnvalue (`GameplayStatics.LoadGameFromSlot` "Settings"))
  (bind _asbp_save_game (cast `/Game/Sound/BP_SaveGame` _returnvalue))
  (set `/Game/Sound/BP_SaveGame.NTries` 3.0 _asbp_save_game)
  (`GameplayStatics.SaveGameToSlot` _asbp_save_game "Settings")
  (bind _returnvalue_2 (`GameplayStatics.GetCurrentLevelName` true))
  (bind _result (`/Engine/EditorBlueprintResources/StandardMacros.IncrementInt` (`KismetArrayLibrary.Array_Find` _levelsname _returnvalue_2))
    (:`  `
      (`GameplayStatics.OpenLevel` (`KismetStringLibrary.Conv_StringToName` (`|GetArrayItem` _levelsname _result))))))

(fn `UserConstructionScript`)